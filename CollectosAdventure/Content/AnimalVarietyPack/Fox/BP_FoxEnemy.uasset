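; BP_FoxEnemy is a fox enemy that chases the player and deals melee-range damage.
; PawnSensing issues an AI MoveTo toward any ThirdPersonCharacter it sees.
; When the player character overlaps DamageBox, a delayed loop repeatedly subtracts a fixed amount directly from the character's CurrentHP.
; The loop has no exit on end overlap or death check, so damage continues after the player leaves the box.
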(event OnSeePawn(PawnSensing)
  (params (Pawn :type Pawn%20Object%20Reference))
  (bind _asthird_person_character (Utilities|Casting|CastToThirdPersonCharacter Pawn))
  (AI|AIMoveTo self "0, 0, 0" _asthird_person_character 5.0 false))

(event OnComponentBeginOverlap(DamageBox)
  (params (OverlappedComponent :type Primitive%20Component%20Object%20Reference) (OtherActor :type Actor%20Object%20Reference) (OtherComp :type Primitive%20Component%20Object%20Reference) (OtherBodyIndex :type Integer) (bFromSweep :type Boolean) (SweepResult :type Hit%20Result%20Structure%20%28by%20ref%29))
  (if (== OtherActor (Game|GetPlayerCharacter 0))
    (Utilities|FlowControl|Delay 0.75 :!label _label)
    (bind _asthird_person_character (Utilities|Casting|CastToThirdPersonCharacter (Game|GetPlayerCharacter 0)))
    (Variables|/Game/ThirdPersonBP/Blueprints/ThirdPersonCharacter.ThirdPersonCharacter_C|SetCurrent%20HP _asthird_person_character (- (Variables|/Game/ThirdPersonBP/Blueprints/ThirdPersonCharacter.ThirdPersonCharacter_C|GetCurrent%20HP _asthird_person_character) 2e+01))
    (Utilities|FlowControl|Delay 0.35)
    (goto _label)))

(event EventBeginPlay)

(event Collision|EventActorBeginOverlap
  (params (OtherActor :type Actor%20Object%20Reference)))

(event EventTick
  (params (DeltaSeconds :type Float%20%28single-precision%29)))

(fn ConstructionScript)